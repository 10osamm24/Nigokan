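; AI character Blueprint with graph sections for random roaming and sensing the player, none of which is functional as wired.
; Tick, FollowPlayer and the construction script are empty.
; Disconnected node chains hold a delayed move to a random reachable point, an AIMoveTo toward the player that prints a debug string, a retriggerable-delayed move to its own location, and a FollowPlayer call.
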(event `self.ReceiveTick`
  (params (DeltaSeconds :type "Float (single-precision)"))
  ;[1 1 1] Random Roam
)

(event `FollowPlayer`
  ;[1 1 1] Sense Player
)

(fn `UserConstructionScript`)