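; AI controller that runs BT_AI on BeginPlay and tracks sight of the first-person player.
; Perception updates drive the "SeePlayer?" blackboard bool, set true half a second after a sighting.
; On losing sight, a retriggerable three-second delay keeps the AI chasing, then rechecks the stimulus before setting or clearing the bool.
; Japanese debug prints mark each perception state.
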(event `self.ReceiveBeginPlay`
  (`self.RunBehaviorTree` "/Game/AI/BT_AI.BT_AI")
  (bind _asbp_ai_character (cast `/Game/AI/BP_AI_Character` (`self.K2_GetPawn`)))
  (set `self.As BP AI Character` _asbp_ai_character))

(event `self.AIPerception.OnTargetPerceptionUpdated`
  (params (Actor :type "Actor Object Reference") (Stimulus :type "AIStimulus Structure"))
  (bind (_age _expirationage _strength _stimuluslocation _receiverlocation _tag _bsuccessfullysensed) (break `AIStimulus` Stimulus))
  (bind _returnvalue (`AIBlueprintHelperLibrary.GetBlackboard` null))
  (cast `/Game/BluePrints/Player/BP_FirstPersonCharacter` Actor)
  (if _bsuccessfullysensed
    (`KismetSystemLibrary.PrintString` "見えた！" true true (struct :`R` 1.0 :`G` 0.071132 :`A` 1.0))
    (`KismetSystemLibrary.Delay` 0.5)
    (`BlackboardComponent.SetValueAsBool` _returnvalue "SeePlayer?" true)
    (else
      (`KismetSystemLibrary.PrintString` "見えなかった！" true true (struct :`R` 1.0 :`G` 0.955324 :`A` 1.0))
      (`KismetSystemLibrary.RetriggerableDelay` 3.0) ; keep chasing for 3 second after lost sight (AI awareness)
      (if _bsuccessfullysensed
        (`KismetSystemLibrary.PrintString` "見つけた！" true true (struct :`R` 1.0 :`G` 0.04875 :`A` 1.0))
        (`BlackboardComponent.SetValueAsBool` _returnvalue "SeePlayer?" true)
        (else
          (`KismetSystemLibrary.PrintString` "見失った！" true true (struct :`R` 0.169409 :`G` 1.0 :`A` 1.0))
          (`BlackboardComponent.SetValueAsBool` _returnvalue "SeePlayer?" false))))))

(fn `UserConstructionScript`)