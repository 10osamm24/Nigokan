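; Enemy character BP_Enemy_Fukui, an AI pawn that moves to locations or a target point and reacts to doors.
; GotoTarget and GoToPoint drive AIMoveTo; hitting a left door clears EnemyOpen if open, or sets it after a delay.
; Box hits against BP_NextFloor enable actor collision, and a getter exposes the four body-part meshes.
; The forward debug RayCast and overlap-based blackboard player sensing are disconnected, the latter with broken casts.
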(event `Go to Target`
  (params (TargetLocation :type "Vector Structure"))
  ;[1 1 1] Move To Target
  (`|AIMoveTo` self TargetLocation null 0.1))

(event `self.Box.OnComponentHit`
  (params (HitComponent :type "PrimitiveComponent Object Reference") (OtherActor :type "Actor Object Reference") (OtherComp :type "PrimitiveComponent Object Reference") (NormalImpulse :type "Vector Structure") (Hit :type "HitResult Structure (by ref)"))
  (cast `/Game/BluePrints/Enviroment/Volumes/BP_NextFloor` OtherActor)
  (`self.SetActorEnableCollision` true))

(event `self.ReceiveHit`
  (params (MyComp :type "PrimitiveComponent Object Reference") (Other :type "Actor Object Reference") (OtherComp :type "PrimitiveComponent Object Reference") (bSelfMoved :type Boolean) (HitLocation :type "Vector Structure") (HitNormal :type "Vector Structure") (NormalImpulse :type "Vector Structure") (Hit :type "HitResult Structure (by ref)"))
  ;[1 1 1] Open door
  (bind _asbp_door_left (cast `/Game/BluePrints/Enviroment/IntaractObjects/BP_Door_Left` Other))
  (if (`/Game/BluePrints/Enviroment/IntaractObjects/BP_Door_Left.isOpen` _asbp_door_left)
    (set `self.EnemyOpen` false)
    (`KismetSystemLibrary.PrintString` "go")
    (else
      (`KismetSystemLibrary.Delay` 2.0)
      (set `self.EnemyOpen` true)
      (`KismetSystemLibrary.PrintString` "open"))))

(event `GoToPoint`
  (`|AIMoveTo` self (0.0 0.0 0.0) (`self.TargetPoint`)))

(fn `GetSkeletalMeshComponent`
  (returns (Body :type "SkeletalMeshComponent Object Reference") (Torso :type "SkeletalMeshComponent Object Reference") (Legs :type "SkeletalMeshComponent Object Reference") (Feet :type "SkeletalMeshComponent Object Reference"))
  (return (`self.Body`) (`self.Torso`) (`self.Legs`) (`self.Feet`)))

(fn `RayCast`
  (returns (HitActor :type "Actor Object Reference"))
  (locals (intaractDistance :type "Float (double-precision)"))
  (bind _mesh (`self.Mesh`))
  (bind _returnvalue (`SceneComponent.K2_GetComponentLocation` _mesh))
  (bind _outhit (`KismetSystemLibrary.LineTraceSingle` :`Start` _returnvalue :`End` (+ _returnvalue (* (`SceneComponent.GetForwardVector` _mesh) (`self.Intaract Distance`))) :`TraceChannel` "TraceTypeQuery1" :`DrawDebugType` "Persistent")) ; レイキャスト
  (return (`.HitActor` (`GameplayStatics.BreakHitResult` _outhit))))

(fn `UserConstructionScript`)