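; BP_FluorescentLight is an environment fluorescent light that starts switched off at BeginPlay.
; TurnOnLight and TurnOffLight each create a dynamic material instance on slot 0 of the FluorescentLight component and set an emissive power scalar from OnLightValue or OffLightValue.
; The two functions use different source materials, and only TurnOffLight takes the parameter name from a variable.
; Nothing in this Blueprint calls TurnOnLight.
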(event `self.ReceiveBeginPlay`
  (`self.TurnOffLight` self))

(event `self.ReceiveTick`
  (params (DeltaSeconds :type "Float (single-precision)")))

(fn `TurnOffLight`
  (bind _returnvalue (`PrimitiveComponent.CreateDynamicMaterialInstance` (`self.FluorescentLight`) 0 "/Game/Assets/Stages/Materials/Emissive/MI_Emmisive.MI_Emmisive" "None"))
  (`MaterialInstanceDynamic.SetScalarParameterValue` _returnvalue (`self.EmmisivePeamName`) (`self.OffLightValue`)))

(fn `TurnOnLight`
  (bind _returnvalue (`PrimitiveComponent.CreateDynamicMaterialInstance` (`self.FluorescentLight`) 0 "/Game/Assets/Stages/Materials/Emissive/M_Emiisive.M_Emiisive" "None"))
  (`MaterialInstanceDynamic.SetScalarParameterValue` _returnvalue "EmmisiivePower" (`self.OnLightValue`)) ; On
)

(fn `UserConstructionScript`)