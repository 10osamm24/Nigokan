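; BP_LoadLightVolume is a trigger volume that shows and hides a configurable set of streaming levels as the first-person character passes through it.
; Exiting the LoadStream component makes each LoadLevel entry visible, while exiting UnloadStream hides the same levels.
; Both paths async-load each world asset to get its name for the streaming-level lookup, then set only ShouldBeVisible.
; The show path also prints each level name.
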(event `self.loadStream.OnComponentEndOverlap`
  (params (OverlappedComponent :type "PrimitiveComponent Object Reference") (OtherActor :type "Actor Object Reference") (OtherComp :type "PrimitiveComponent Object Reference") (OtherBodyIndex :type Integer))
  (cast `/Game/BluePrints/Player/BP_FirstPersonCharacter` OtherActor)
  (for _array_element (`self.LoadLevel`)
    (bind _object (`|LoadAsset` (`.WorldAsset` (break `SoftWorldReference` _array_element))) ; Stringに変換
      (:`Completed`
        (bind _returnvalue (`KismetStringLibrary.Conv_StringToName` (`KismetSystemLibrary.GetObjectName` _object)))
        (set `LevelStreaming.bShouldBeVisible` true (`GameplayStatics.GetStreamingLevel` _returnvalue)) ; 可視化
        (`KismetSystemLibrary.PrintString` (`KismetStringLibrary.Conv_NameToString` _returnvalue))))))

(event `self.UnloadStream.OnComponentEndOverlap`
  (params (OverlappedComponent :type "PrimitiveComponent Object Reference") (OtherActor :type "Actor Object Reference") (OtherComp :type "PrimitiveComponent Object Reference") (OtherBodyIndex :type Integer))
  (cast `/Game/BluePrints/Player/BP_FirstPersonCharacter` OtherActor)
  (for _array_element (`self.LoadLevel`)
    (bind _object (`|LoadAsset` (`.WorldAsset` (break `SoftWorldReference` _array_element))) ; Stringに変換
      (:`Completed`
        (set `LevelStreaming.bShouldBeVisible` false (`GameplayStatics.GetStreamingLevel` (`KismetStringLibrary.Conv_StringToName` (`KismetSystemLibrary.GetObjectName` _object)))) ; 非可視化
      ))))

(fn `UserConstructionScript`)