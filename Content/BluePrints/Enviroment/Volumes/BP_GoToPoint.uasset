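; BP_GoToPoint is a trigger volume that records which floor the player is on and sends the AI toward a point.
; When BP_FirstPersonCharacter overlaps its collision component, it copies the volume's CurFloor into the character's CurrentFloor.
; Three sequenced checks compare that value to E_Floor entries; a match prints a debug number and calls GoToPoint on the BP_AIController found through GetActorOfClass.
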(event `self.CollisionComponent.OnComponentBeginOverlap`
  (params (OverlappedComponent :type "PrimitiveComponent Object Reference") (OtherActor :type "Actor Object Reference") (OtherComp :type "PrimitiveComponent Object Reference") (OtherBodyIndex :type Integer) (bFromSweep :type Boolean) (SweepResult :type "HitResult Structure (by ref)"))
  (bind _asbp_first_person_character (cast `/Game/BluePrints/Player/BP_FirstPersonCharacter` OtherActor))
  (`|ExecutionSequence`
    (:`then_0`
      (bind _output_get (set `/Game/BluePrints/Player/BP_FirstPersonCharacter.CurrentFloor` (`self.CurFloor`) _asbp_first_person_character))
      (if (== _output_get (`KismetMathLibrary.Conv_ByteToInt` (enumliteral `/Game/BluePrints/Enviroment/Volumes/E_Floor` "NewEnumerator0")))
        (`KismetSystemLibrary.PrintString` "1")
        (bind _returnvalue (`GameplayStatics.GetActorOfClass` "/Game/BluePrints/Enemy/BP_AIController.BP_AIController_C"))
        (`/Game/BluePrints/Enemy/BP_AIController.GoToPoint` _returnvalue)))
    (:`then_1`
      (bind _output_get_2 (set `/Game/BluePrints/Player/BP_FirstPersonCharacter.CurrentFloor` (`self.CurFloor`) _asbp_first_person_character))
      (if (== _output_get_2 (`KismetMathLibrary.Conv_ByteToInt` (enumliteral `/Game/BluePrints/Enviroment/Volumes/E_Floor` "NewEnumerator1")))
        (`KismetSystemLibrary.PrintString` "2")
        (bind _returnvalue_2 (`GameplayStatics.GetActorOfClass` "/Game/BluePrints/Enemy/BP_AIController.BP_AIController_C"))
        (`/Game/BluePrints/Enemy/BP_AIController.GoToPoint` _returnvalue_2)))
    (:`then_2`
      (bind _output_get_3 (set `/Game/BluePrints/Player/BP_FirstPersonCharacter.CurrentFloor` (`self.CurFloor`) _asbp_first_person_character))
      (if (== _output_get_3 (`KismetMathLibrary.Conv_ByteToInt` (enumliteral `/Game/BluePrints/Enviroment/Volumes/E_Floor` "NewEnumerator2")))
        (`KismetSystemLibrary.PrintString` "3")
        (bind _returnvalue_3 (`GameplayStatics.GetActorOfClass` "/Game/BluePrints/Enemy/BP_AIController.BP_AIController_C"))
        (`/Game/BluePrints/Enemy/BP_AIController.GoToPoint` _returnvalue_3)))))

(fn `UserConstructionScript`)