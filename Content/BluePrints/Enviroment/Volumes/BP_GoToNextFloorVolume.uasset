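; Trigger volume that records which floor the player and the Fukui enemy are on and sends the AI after the player.
; On player overlap it sets the character's CurrentFloor from CurFloorPlayerBox and passes that floor to BP_AIController's GoToPoint.
; On enemy overlap it sets the enemy's CurrentFloor from CurFloorEnemyBox.
; Older per-floor comparisons with debug prints remain in the graph but never run.
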(event `self.CollisionComponent.OnComponentBeginOverlap`
  (params (OverlappedComponent :type "PrimitiveComponent Object Reference") (OtherActor :type "Actor Object Reference") (OtherComp :type "PrimitiveComponent Object Reference") (OtherBodyIndex :type Integer) (bFromSweep :type Boolean) (SweepResult :type "HitResult Structure (by ref)"))
  (bind _curfloor_playerbox (`self.CurFloor_PlayerBox`))
  (`|ExecutionSequence`
    (:`then_0`
      (bind _asbp_first_person_character (cast `/Game/BluePrints/Player/BP_FirstPersonCharacter` OtherActor))
      (set `/Game/BluePrints/Player/BP_FirstPersonCharacter.CurrentFloor` _curfloor_playerbox _asbp_first_person_character)
      (bind _returnvalue (`GameplayStatics.GetActorOfClass` "/Game/BluePrints/Enemy/BP_AIController.BP_AIController_C"))
      (`/Game/BluePrints/Enemy/BP_AIController.GoToPoint` _returnvalue _curfloor_playerbox))
    (:`then_1`
      (bind _asbp_enemy_fukui (cast `/Game/BluePrints/Enemy/Fukui/BP_Enemy_Fukui` OtherActor))
      (bind _output_get (set `/Game/BluePrints/Enemy/Fukui/BP_Enemy_Fukui.CurrentFloor` (`self.CurFloor_EnemyBox`) _asbp_enemy_fukui))
      (switch `/Game/BluePrints/Enviroment/Volumes/E_Floor` _output_get))))

(fn `UserConstructionScript`)