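; BP_NextFloorBlockVolume is a volume that toggles whether pawns can pass, apparently gating access to the next floor.
; When the first-person character hits its collision component, the Pawn channel response switches to Overlap, opening the volume.
; An overlap by BP_Enemy_Fukui starts a retriggerable delay of a few seconds, after which the response returns to Block.
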(event `self.CollisionComponent.OnComponentHit`
  (params (HitComponent :type "PrimitiveComponent Object Reference") (OtherActor :type "Actor Object Reference") (OtherComp :type "PrimitiveComponent Object Reference") (NormalImpulse :type "Vector Structure") (Hit :type "HitResult Structure (by ref)"))
  (cast `/Game/BluePrints/Player/BP_FirstPersonCharacter` OtherActor)
  (set `self.onHit` true)
  (if (`self.onHit`)
    (`PrimitiveComponent.SetCollisionResponseToChannel` (`self.CollisionComponent`) "ECC_Pawn" "ECR_Overlap")))

(event `self.CollisionComponent.OnComponentBeginOverlap`
  (params (OverlappedComponent :type "PrimitiveComponent Object Reference") (OtherActor :type "Actor Object Reference") (OtherComp :type "PrimitiveComponent Object Reference") (OtherBodyIndex :type Integer) (bFromSweep :type Boolean) (SweepResult :type "HitResult Structure (by ref)"))
  (cast `/Game/BluePrints/Enemy/Fukui/BP_Enemy_Fukui` OtherActor)
  (`KismetSystemLibrary.RetriggerableDelay` 3.0)
  (set `self.onHit` false)
  (if (not (`self.onHit`))
    (`PrimitiveComponent.SetCollisionResponseToChannel` (`self.CollisionComponent`) "ECC_Pawn" "ECR_Block")))

(fn `UserConstructionScript`)