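; BP_RoomVolume is a room volume that tells the player character and enemies which room they are in.
; On begin overlap, it writes its RoomNumber into the CurrentRoomNumber of an overlapping BP_FirstPersonCharacter or BP_Enemy.
; On end overlap, it unconditionally resets that value to the 9999 sentinel, even if the actor has already entered another room volume.
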(event `self.ReceiveActorBeginOverlap`
  (params (OtherActor :type "Actor Object Reference"))
  (`|ExecutionSequence`
    (:`then_0`
      (bind _asbp_first_person_character (cast `/Game/BluePrints/Player/BP_FirstPersonCharacter` OtherActor))
      (set `/Game/BluePrints/Player/BP_FirstPersonCharacter.CurrentRoomNumber` (`self.RoomNumber`) _asbp_first_person_character))
    (:`then_1`
      (bind _asbp_enemy (cast `/Game/BluePrints/Enemy/BP_Enemy` OtherActor))
      (set `/Game/BluePrints/Enemy/BP_Enemy.CurrentRoomNumber` (`self.RoomNumber`) _asbp_enemy))))

(event `self.ReceiveActorEndOverlap`
  (params (OtherActor :type "Actor Object Reference"))
  (`|ExecutionSequence`
    (:`then_0`
      (bind _asbp_first_person_character (cast `/Game/BluePrints/Player/BP_FirstPersonCharacter` OtherActor))
      (set `/Game/BluePrints/Player/BP_FirstPersonCharacter.CurrentRoomNumber` 9999 _asbp_first_person_character))
    (:`then_1`
      (bind _asbp_enemy (cast `/Game/BluePrints/Enemy/BP_Enemy` OtherActor))
      (set `/Game/BluePrints/Enemy/BP_Enemy.CurrentRoomNumber` 9999 _asbp_enemy))))

(fn `UserConstructionScript`)