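; Tutorial UI volume that drives the in-game HUD's tutorial event from its collision component.
; A hit on the component passes the volume's TutorialType to HUD_InGame, found through player controller 0.
; End overlap switches the HUD to a fixed tutorial enum value and destroys the volume.
; Neither event filters the other actor, and the show trigger uses component hit rather than begin overlap.
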(event `self.CollisionComponent.OnComponentHit`
  (params (HitComponent :type "PrimitiveComponent Object Reference") (OtherActor :type "Actor Object Reference") (OtherComp :type "PrimitiveComponent Object Reference") (NormalImpulse :type "Vector Structure") (Hit :type "HitResult Structure (by ref)"))
  (bind _ashud_in_game (cast `/Game/BluePrints/Framework/GameModes/HUD_InGame` (`PlayerController.GetHUD` (`GameplayStatics.GetPlayerController` 0))))
  (`/Game/BluePrints/Framework/GameModes/HUD_InGame.SetTutorial_Event` _ashud_in_game (`self.tutorialType`)))

(event `self.CollisionComponent.OnComponentEndOverlap`
  (params (OverlappedComponent :type "PrimitiveComponent Object Reference") (OtherActor :type "Actor Object Reference") (OtherComp :type "PrimitiveComponent Object Reference") (OtherBodyIndex :type Integer))
  (bind _ashud_in_game (cast `/Game/BluePrints/Framework/GameModes/HUD_InGame` (`PlayerController.GetHUD` (`GameplayStatics.GetPlayerController` 0))))
  (`/Game/BluePrints/Framework/GameModes/HUD_InGame.SetTutorial_Event` _ashud_in_game "NewEnumerator7")
  (`self.K2_DestroyActor`))

(fn `UserConstructionScript`)