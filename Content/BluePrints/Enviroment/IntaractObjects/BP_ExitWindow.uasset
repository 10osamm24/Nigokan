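; BP_ExitWindow is an interactable escape window that the player breaks, fits with a rope ladder and uses to clear the game.
; Interacting consumes an item to break it or, once the rope is set, calls GameClearEvent on the game mode.
; Holding interact with the rope item accumulates Tick delta time into a gauge widget, then reveals the Rope.
; Looking at it updates the Japanese action prompt from progress and held items.
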(event `self.ReceiveBeginPlay`
  ;[1 1 1] 初期化処理
  (`parent.ReceiveBeginPlay`)
  (bind _returnvalue (`|CreateWidget` "/Game/BluePrints/UI/InGame/BPW_SetRopeGame.BPW_SetRopeGame_C"))
  (bind _output_get (set `self.BPW_Gage` _returnvalue))
  (`UserWidget.AddToViewport` _output_get 0)
  (`Widget.SetVisibility` (`self.BPW_Gage`) "Collapsed"))

(event `self.IntaractAction_Event`
  ;[1 1 1] インタラクト処理
  (if (`self.isSetRope`)
    ;;[1 1 1] ゲームクリア
    (bind _asbp_first_person_game_mode (cast `/Game/BluePrints/Framework/GameModes/BP_FirstPersonGameMode` (`GameplayStatics.GetGameMode`)))
    (`/Game/BluePrints/Framework/GameModes/BP_FirstPersonGameMode.GameClear_Event` _asbp_first_person_game_mode)
    (else
      (bind _asbp_first_person_character (cast `/Game/BluePrints/Player/BP_FirstPersonCharacter` (`GameplayStatics.GetPlayerCharacter` 0)))
      (if (not (`self.isBrokeWindow`))
        ;;[1 1 1] 窓を壊す
        (bind _iscanuse (`/Game/BluePrints/Player/BP_FirstPersonCharacter.UseItem` _asbp_first_person_character "NewEnumerator3"))
        (if _iscanuse
          (set `self.isBrokeWindow` true))))))

(event `self.ReceiveTick`
  (params (DeltaSeconds :type "Float (single-precision)"))
  ;[1 1 1] 更新処理
  (`parent.ReceiveTick` DeltaSeconds)
  (set `self.DeltaTime` DeltaSeconds))

(event `self.HoldUpdate_Event`
  ;[1 1 1] 長押し処理
  (bind _asbp_first_person_character (cast `/Game/BluePrints/Player/BP_FirstPersonCharacter` (`GameplayStatics.GetPlayerCharacter` 0)))
  (if (> (`|GetArrayItem` (`/Game/BluePrints/Player/BP_FirstPersonCharacter.HoldItems` _asbp_first_person_character) (`KismetMathLibrary.Conv_ByteToInt` (enumliteral `/Game/BluePrints/Enviroment/Items/E_Item` "NewEnumerator4"))) 0)
    (if (`self.isBrokeWindow`)
      (if (>= (`self.ropeSetTime`) (`self.ROPE_SET_TIME`))
        ;;[1 1 1] ロープを設置
        (bind _iscanuse (`/Game/BluePrints/Player/BP_FirstPersonCharacter.UseItem` _asbp_first_person_character "NewEnumerator4"))
        (if _iscanuse
          (set `self.isSetRope` true)
          (`SceneComponent.SetVisibility` (`self.Rope`) true false)
          (`Widget.SetVisibility` (`self.BPW_Gage`) "Collapsed") ; ゲージを非表示する
        )
        (else
          ;;[1 1 1] 時間経過
          (bind _output_get (set `self.ropeSetTime` (+ (`self.ropeSetTime`) (`self.DeltaTime`))))
          (`/Game/BluePrints/UI/InGame/BPW_SetRopeGame.Set Parsent` (`self.BPW_Gage`) (/ _output_get (`self.ROPE_SET_TIME`)))
          (`Widget.SetVisibility` (`self.BPW_Gage`) "Visible") ; ゲージを表示する
        )))))

(event `self.HoldComplete_Event`
  (`Widget.SetVisibility` (`self.BPW_Gage`) "Collapsed") ; ゲージを非表示する
)

(event `self.OnLooking_Event`
  (if (>= (`self.ropeSetTime`) (`self.ROPE_SET_TIME`))
    (set `self.actionName` "脱出する")
    (elif (`self.isBrokeWindow`)
      (bind _asbp_first_person_character (cast `/Game/BluePrints/Player/BP_FirstPersonCharacter` (`GameplayStatics.GetPlayerCharacter` 0)))
      (if (> (`|GetArrayItem` (`/Game/BluePrints/Player/BP_FirstPersonCharacter.HoldItems` _asbp_first_person_character) (`KismetMathLibrary.Conv_ByteToInt` (enumliteral `/Game/BluePrints/Enviroment/Items/E_Item` "NewEnumerator4"))) 0)
        (set `self.actionName` "はしごを置く(長押し)")
        (else
          (set `self.actionName` "割れた窓")))
      (else
        (bind _asbp_first_person_character_2 (cast `/Game/BluePrints/Player/BP_FirstPersonCharacter` (`GameplayStatics.GetPlayerCharacter` 0)))
        (if (> (`|GetArrayItem` (`/Game/BluePrints/Player/BP_FirstPersonCharacter.HoldItems` _asbp_first_person_character_2) (`KismetMathLibrary.Conv_ByteToInt` (enumliteral `/Game/BluePrints/Enviroment/Items/E_Item` "NewEnumerator3"))) 0)
          (set `self.actionName` "窓を割る"))))))

(fn `UserConstructionScript`
  (`parent.UserConstructionScript`))