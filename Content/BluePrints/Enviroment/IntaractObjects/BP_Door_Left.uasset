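; BP_Door_Left is an interactable door that toggles open and closed, with a Japanese action label reflecting the next action.
; The DoorAngle timeline plays or reverses to drive the yaw of Object, then snaps the interaction range back to IntaractPos when finished.
; The door sound plays as opening starts and when closing completes.
; A hit from BP_Enemy_Fukui with EnemyOpen set also triggers the opening branch.
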(event `self.ReceiveBeginPlay`
  (`parent.ReceiveBeginPlay`)
  (`SceneComponent.K2_SetWorldLocation` (`self.IntaractRounge`) (`SceneComponent.K2_GetComponentLocation` (`self.intaractPos`)) false false)
  (set `self.actionName` "開ける"))

(event `self.ReceiveTick`
  (params (DeltaSeconds :type "Float (single-precision)"))
  (`parent.ReceiveTick` DeltaSeconds))

(event `self.IntaractAction_Event`
  (if (`self.isOpen`)
    (set `self.isOpen` false) ; ドアを開けウr
    (set `self.actionName` "開ける")
    (bind (_direction _doorangle) (`Timeline|doorAngle` :`NewTime` 0.5 :!via `Reverse` :!label _label)
      (:`Update`
        (`SceneComponent.K2_SetRelativeRotation` (`self.Object`) (`KismetMathLibrary.MakeRotator` 0.0 0.0 _doorangle) false false))
      (:`Finished`
        (`SceneComponent.K2_SetWorldLocation` (`self.IntaractRounge`) (`SceneComponent.K2_GetComponentLocation` (`self.intaractPos`)) false false)
        ;[1 1 1] 閉めた音
        (if (not (`self.isOpen`))
          (`GameplayStatics.PlaySoundAtLocation` (`self.doorSound`) (0.0 0.0 0.0) (struct) 1.0 1.0 0.47 null null null null))))
    (else
      (set `self.isOpen` true :!label _label_2) ; ドアを開ける
      (set `self.actionName` "閉める")
      (`GameplayStatics.PlaySoundAtLocation` (`self.doorSound`) (0.0 0.0 0.0) (struct) 1.0 1.0 0.5 null null null null)
      (goto _label))))

(event `self.ReceiveHit`
  (params (MyComp :type "PrimitiveComponent Object Reference") (Other :type "Actor Object Reference") (OtherComp :type "PrimitiveComponent Object Reference") (bSelfMoved :type Boolean) (HitLocation :type "Vector Structure") (HitNormal :type "Vector Structure") (NormalImpulse :type "Vector Structure") (Hit :type "HitResult Structure (by ref)"))
  (bind _asbp_enemy_fukui (cast `/Game/BluePrints/Enemy/Fukui/BP_Enemy_Fukui` Other))
  (if (`/Game/BluePrints/Enemy/Fukui/BP_Enemy_Fukui.EnemyOpen` _asbp_enemy_fukui)
    (goto _label_2)))

(fn `UserConstructionScript`
  (`parent.UserConstructionScript`))