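; BP_Door_Right is an interactable door that toggles open and closed when MoveDoor_Event is called.
; The event flips IsOpen and plays or reverses the DoorAngle timeline, which sets the relative yaw of Object.
; IntaractRounge snaps to the IntaractPos world location at BeginPlay and when the timeline finishes, keeping the interaction range aligned with the door.
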(event `self.ReceiveBeginPlay`
  (`parent.ReceiveBeginPlay`)
  (`SceneComponent.K2_SetWorldLocation` (`self.IntaractRounge`) (`SceneComponent.K2_GetComponentLocation` (`self.intaractPos`)) false false))

(event `self.ReceiveTick`
  (params (DeltaSeconds :type "Float (single-precision)"))
  (`parent.ReceiveTick` DeltaSeconds))

(event `MoveDoor_Event`
  (if (`self.isOpen`)
    (set `self.isOpen` false)
    (bind (_direction _doorangle) (`Timeline|doorAngle` :`NewTime` 0.5 :!via `Reverse` :!label _label)
      (:`Update`
        (`SceneComponent.K2_SetRelativeRotation` (`self.Object`) (`KismetMathLibrary.MakeRotator` 0.0 0.0 _doorangle) false false))
      (:`Finished`
        (`SceneComponent.K2_SetWorldLocation` (`self.IntaractRounge`) (`SceneComponent.K2_GetComponentLocation` (`self.intaractPos`)) false false)))
    (else
      (set `self.isOpen` true)
      (goto _label))))

(fn `UserConstructionScript`
  (`parent.UserConstructionScript`))