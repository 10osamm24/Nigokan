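; Parent Blueprint for an interactable hinged door that the interact event opens or closes unless it is locked.
; Two timelines drive the door's yaw, chosen by ObjType for swing direction, with sounds and an updated action label.
; The interaction range snaps to its anchor when a swing finishes, and BeginPlay fires the interact event once.
; A BP_Enemy_Fukui hit with EnemyOpen false opens the door, bypassing the lock.
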(event `self.ReceiveBeginPlay`
  (`parent.ReceiveBeginPlay`)
  (`SceneComponent.K2_SetWorldLocation` (`self.IntaractRounge`) (`SceneComponent.K2_GetComponentLocation` (`self.intaractPos`)) false false)
  (`self.IntaractAction_Event`) ; 開始直後に占める
)

(event `self.IntaractAction_Event`
  (bind _returnvalue (== (enumliteral `/Game/BluePrints/Enviroment/IntaractObjects/E_IntaractObjType` "NewEnumerator0") (`KismetMathLibrary.Conv_ByteToInt` (`self.objType`))))
  (if (`self.isLooked`)
    (set `self.actionName` "開かない")
    (elif (`self.isOpen`)
      (set `self.isOpen` false)
      (set `self.actionName` "開ける")
      (if _returnvalue
        (bind (_direction _doorangle) (`Timeline|タイムライン` :`NewTime` 0.5 :!via `Reverse` :!label _label) ; ➤
          (:`Update`
            (`SceneComponent.K2_SetRelativeRotation` (`self.Object`) (`KismetMathLibrary.MakeRotator` 0.0 0.0 _doorangle) false false))
          (:`Finished`
            (`SceneComponent.K2_SetWorldLocation` (`self.IntaractRounge`) (`SceneComponent.K2_GetComponentLocation` (`self.intaractPos`)) false false :!label _label_2)
            ;[1 1 1] 閉めた音
            (if (not (`self.isOpen`))
              (`GameplayStatics.PlaySoundAtLocation` (`self.doorSound`) (0.0 0.0 0.0) (struct) 1.0 1.0 0.47 null null null null))))
        (else
          (bind (_direction_2 _doorangle_2) (`Timeline|タイムライン_0` :`NewTime` 0.5 :!via `Reverse` :!label _label_3) ; 左
            (:`Update`
              (`SceneComponent.K2_SetRelativeRotation` (`self.Object`) (`KismetMathLibrary.MakeRotator` 0.0 0.0 _doorangle_2) false false))
            (:`Finished`
              (goto _label_2)))))
      (else
        (set `self.isOpen` true :!label _label_4)
        (set `self.actionName` "閉める")
        (`GameplayStatics.PlaySoundAtLocation` (`self.doorSound`) (0.0 0.0 0.0) (struct) 1.0 1.0 0.5 null null null null)
        (if _returnvalue
          (goto _label)
          (else
            (goto _label_3)))))))

(event `self.Object.OnComponentHit`
  (params (HitComponent :type "PrimitiveComponent Object Reference") (OtherActor :type "Actor Object Reference") (OtherComp :type "PrimitiveComponent Object Reference") (NormalImpulse :type "Vector Structure") (Hit :type "HitResult Structure (by ref)"))
  (bind _asbp_enemy_fukui (cast `/Game/BluePrints/Enemy/Fukui/BP_Enemy_Fukui` OtherActor))
  (if (not (`/Game/BluePrints/Enemy/Fukui/BP_Enemy_Fukui.EnemyOpen` _asbp_enemy_fukui))
    (goto _label_4)))

(event `UnLook_Event`
  (set `self.isLooked` false))

(fn `UserConstructionScript`
  (`parent.UserConstructionScript`))