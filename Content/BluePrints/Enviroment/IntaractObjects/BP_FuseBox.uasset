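; BP_FuseBox is an interactable environment fuse box that shows fuses as they are inserted.
; Each SetFuse_Event call, while FuseCount is below MAXFUSENUM, switches on the count to reveal the next of three fuse components, then increments the count.
; The event only updates visibility and the count, with no completion logic in this graph.
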(event `SetFuse_Event`
  (if (not (>= (`self.fuseCount`) (`self.MAX_FUSE_NUM`)))
    (switch `int` (`self.fuseCount`)
      (:`0`
        ;[1 1 1] ヒューズを表示する
        (`SceneComponent.SetVisibility` (`self.Fuse`) true false))
      (:`1`
        (`SceneComponent.SetVisibility` (`self.Fuse1`) true false))
      (:`2`
        (`SceneComponent.SetVisibility` (`self.Fuse2`) true false)))
    ;[1 1 1] 所持数を加算
    (`/Engine/EditorBlueprintResources/StandardMacros.IncrementInt` (`self.fuseCount`))))

(fn `UserConstructionScript`
  (`parent.UserConstructionScript`))