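; Interactable charging dock where the player places a held phone, waits for it to charge, then calls the police to start a timed escape ending in game clear.
; The interact event consumes the phone item or starts the countdown, while the look event sets the state-dependent action prompt.
; Tick advances the charge, lighting the phone's dynamic emissive material when full, then drives the timer widget and calls the GameMode's clear event at zero.
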(event `self.ReceiveBeginPlay`
  (bind _phone (`self.phone`))
  ;[1 1 1] 初期化処理
  (`parent.ReceiveBeginPlay`)
  (bind _returnvalue (`PrimitiveComponent.CreateDynamicMaterialInstance` _phone 0 (`PrimitiveComponent.GetMaterial` _phone 0) "None"))
  (bind _output_get (set `self.Emmisive` _returnvalue))
  (`MaterialInstanceDynamic.SetScalarParameterValue` _output_get "EmmisiivePower" 0.0)
  (`MaterialInstanceDynamic.SetScalarParameterValue` _returnvalue "EmmisiivePower" 0.0)
  ;;[1 1 1] タイマーUI初期化
  (bind _returnvalue_2 (`|CreateWidget` "/Game/BluePrints/UI/InGame/BPW_Escape3_Timer.BPW_Escape3_Timer_C"))
  (bind _output_get_2 (set `self.TimerWBP` _returnvalue_2))
  (`UserWidget.AddToViewport` _output_get_2 0)
  (`Widget.SetVisibility` _output_get_2 "Collapsed"))

(event `self.IntaractAction_Event`
  (if (`self.isSetPhone`)
    ;[1 1 1] 警察を呼ぶ
    (if (`self.isEnableEscape`)
      (`/Engine/EditorBlueprintResources/StandardMacros.DoOnce` false
        (:`Completed`
          (set `self.isEscapeTImer` true)
          (`Widget.SetVisibility` (`self.TimerWBP`) "Visible")
          (set `self.EscapeTimer` (`self.ESCAPE_TIME`)) ; タイマーをセット
        )))
    (else
      ;[1 1 1] 携帯を設置する
      (`/Engine/EditorBlueprintResources/StandardMacros.DoOnce` false
        (:`Completed`
          (bind _asbp_first_person_character (cast `/Game/BluePrints/Player/BP_FirstPersonCharacter` (`GameplayStatics.GetPlayerCharacter` 0)))
          (bind _iscanuse (`/Game/BluePrints/Player/BP_FirstPersonCharacter.UseItem` _asbp_first_person_character "NewEnumerator6"))
          (if _iscanuse
            (set `self.isSetPhone` true)
            (`SceneComponent.SetVisibility` (`self.Phone`) true false) ; 携帯を表示
          ))))))

(event `self.OnLooking_Event`
  ;[1 1 1] 状態によって表示するＡｃｔｉｏｎＮａｍｅが変わる
  (if (`self.isSetPhone`)
    (if (>= (`self.chargeTimer`) (`self.CHARGE_TIME`))
      (set `self.actionName` "警察を呼ぶ")
      (else
        (set `self.actionName` (`KismetStringLibrary.Concat_StrStr` "充電完了まで" "（" (`KismetStringLibrary.Conv_Int64ToString` (`KismetMathLibrary.Conv_DoubleToInt64` (`KismetMathLibrary.Lerp` 0.0 10.0 (- (`self.CHARGE_TIME`) (`self.chargeTimer`))))) "％）"))))
    (else
      (bind _asbp_first_person_character (cast `/Game/BluePrints/Player/BP_FirstPersonCharacter` (`GameplayStatics.GetPlayerCharacter` 0)))
      (if (> (`|GetArrayItem` (`/Game/BluePrints/Player/BP_FirstPersonCharacter.HoldItems` _asbp_first_person_character) (`KismetMathLibrary.Conv_ByteToInt` (enumliteral `/Game/BluePrints/Enviroment/Items/E_Item` "NewEnumerator6"))) 0)
        (set `self.actionName` "充電する")))))

(event `self.ReceiveTick`
  (params (DeltaSeconds :type "Float (single-precision)"))
  (bind _escapetimer (`self.EscapeTimer`))
  (bind _returnvalue (`KismetMathLibrary.Conv_IntToDouble` (/ _escapetimer 60)))
  (`parent.ReceiveTick` DeltaSeconds)
  (if (`self.isEscapeTImer`)
    ;[1 1 1] 逃げる時間経過
    (if (>= 0.0 (`self.EscapeTimer`))
      ;[1 1 1] ゲームクリア
      (bind _asbp_first_person_game_mode (cast `/Game/BluePrints/Framework/GameModes/BP_FirstPersonGameMode` (`GameplayStatics.GetGameMode`)))
      (`/Game/BluePrints/Framework/GameModes/BP_FirstPersonGameMode.GameClear_Event` _asbp_first_person_game_mode)
      (else
        (set `self.EscapeTimer` (- (`self.EscapeTimer`) DeltaSeconds))
        (`/Game/BluePrints/UI/InGame/BPW_Escape3_Timer.SetTimer_Event` (`self.TimerWBP`) _returnvalue (- _escapetimer (* _returnvalue 60.0)))))
    (else
      ;[1 1 1] 充電時間更新
      (if (`self.isSetPhone`)
        (if (>= (`self.chargeTimer`) (`self.CHARGE_TIME`))
          (`/Engine/EditorBlueprintResources/StandardMacros.DoOnce` false
            (:`Completed`
              (`MaterialInstanceDynamic.SetScalarParameterValue` (`self.Emmisive`) "EmmisiivePower" 10.0)
              (set `self.isEnableEscape` true)))
          (else
            (set `self.chargeTimer` (+ DeltaSeconds (`self.chargeTimer`)))))))))

(fn `UserConstructionScript`
  (`parent.UserConstructionScript`))