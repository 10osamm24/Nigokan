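; Interactable fuse box of a set color that the player fills with a matching fuse.
; On interaction it maps FuseColor to an item, consumes it through the character's UseItem, shows the Fuse mesh, plays a sound and notifies the game mode via SetFuseBoxEvent.
; When looked at, it updates the Japanese ActionName prompt from a fixed item count, independent of color, or from the fuse's visibility.
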(event `self.ReceiveBeginPlay`
  (`parent.ReceiveBeginPlay`)
  (set `self.actionName` (`KismetStringLibrary.Concat_StrStr` "ヒューズボックス" "（" (`|GetEnumeratorNameAsString` (`self.fuseColor`)) "）")))

(event `self.IntaractAction_Event`
  ;[1 1 1] ヒューズを設置
  (bind _asbp_first_person_character (cast `/Game/BluePrints/Player/BP_FirstPersonCharacter` (`GameplayStatics.GetPlayerCharacter` 0)))
  (bind _itemtype (`self.GetFuseColor`))
  (bind _iscanuse (`/Game/BluePrints/Player/BP_FirstPersonCharacter.UseItem` _asbp_first_person_character _itemtype))
  (if _iscanuse
    (`SceneComponent.SetVisibility` (`self.Fuse`) true false) ; ヒューズを表示
    (`GameplayStatics.PlaySoundAtLocation` "/Game/Assets/Sounds/Effect/Fuse-set.Fuse-set" (0.0 0.0 0.0) (struct) 1.0 1.0 0.0 null null null null) ; 設置音再生
    (bind _asbp_first_person_game_mode (cast `/Game/BluePrints/Framework/GameModes/BP_FirstPersonGameMode` (`GameplayStatics.GetGameMode`)))
    (`/Game/BluePrints/Framework/GameModes/BP_FirstPersonGameMode.SetFuseBox_Event` _asbp_first_person_game_mode (`self.fuseColor`))))

(event `self.OnLooking_Event`
  (bind _asbp_first_person_character (cast `/Game/BluePrints/Player/BP_FirstPersonCharacter` (`GameplayStatics.GetPlayerCharacter` 0)))
  (if (> (`|GetArrayItem` (`/Game/BluePrints/Player/BP_FirstPersonCharacter.HoldItems` _asbp_first_person_character) (`KismetMathLibrary.Conv_ByteToInt` (enumliteral `/Game/BluePrints/Enviroment/Items/E_Item` "NewEnumerator1"))) 0)
    (set `self.actionName` "ヒューズを入れる")
    (elif (`SceneComponent.IsVisible` (`self.Fuse`))
      (set `self.actionName` (`KismetStringLibrary.Concat_StrStr` "設置済みのヒューズボックス" "（" (`|GetEnumeratorNameAsString` (`self.fuseColor`)) "）"))
      (else
        (set `self.actionName` (`KismetStringLibrary.Concat_StrStr` "ヒューズボックス" "（" (`|GetEnumeratorNameAsString` (`self.fuseColor`)) "）"))))))

(fn `GetFuseColor`
  (returns (itemType :type "/Game/BluePrints/Enviroment/Items/E_Item Enum"))
  (switch `/Game/BluePrints/Enviroment/IntaractObjects/Fuse/E_FuseColor` (`self.fuseColor`)
    (:`NewEnumerator0`
      (return "NewEnumerator7"))
    (:`NewEnumerator1`
      (return "NewEnumerator9"))
    (:`NewEnumerator2`
      (return "NewEnumerator8"))))

(fn `UserConstructionScript`
  (`parent.UserConstructionScript`))