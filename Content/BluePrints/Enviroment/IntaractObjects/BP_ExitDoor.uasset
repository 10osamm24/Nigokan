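; BP_ExitDoor is the double exit door that opens once all three fuses are set and serves as the game's clear point.
; Tick polls the game mode's fuse array, then plays chained timelines once to swing the right and left doors.
; The left door's first update also destroys IntaractMesh.
; When the player character overlaps ClearBox, it calls GameClearEvent on the game mode.
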(event `self.ReceiveBeginPlay`
  (`parent.ReceiveBeginPlay`))

(event `self.ReceiveTick`
  (params (DeltaSeconds :type "Float (single-precision)"))
  (`parent.ReceiveTick` DeltaSeconds)
  ;[1 1 1] 扉を開く
  (bind _asbp_first_person_game_mode (cast `/Game/BluePrints/Framework/GameModes/BP_FirstPersonGameMode` (`GameplayStatics.GetGameMode`)))
  (if (`KismetArrayLibrary.Array_Identical` (`/Game/BluePrints/Framework/GameModes/BP_FirstPersonGameMode.isSetAllFuse` _asbp_first_person_game_mode) (`|MakeArray` true true true))
    (`/Engine/EditorBlueprintResources/StandardMacros.DoOnce` false
      (:`Completed`
        ;;[1 1 1] 右の扉を開く
        (bind (_direction _doorangle) (`Timeline|タイムライン` :`NewTime` 0.5)
          (:`Update`
            (`SceneComponent.K2_SetRelativeRotation` (`self.DoorRight`) (`KismetMathLibrary.MakeRotator` 0.0 0.0 _doorangle) false false)
            ;;[1 1 1] 左の扉を開く
            (bind (_direction_2 _doorangle_2) (`Timeline|タイムライン_0` :`NewTime` 0.5)
              (:`Update`
                (`SceneComponent.K2_SetRelativeRotation` (`self.DoorLeft`) (`KismetMathLibrary.MakeRotator` 0.0 0.0 _doorangle_2) false false)
                (`/Engine/EditorBlueprintResources/StandardMacros.DoOnce` false
                  (:`Completed`
                    (`ActorComponent.K2_DestroyComponent` (`self.IntaractMesh`))))))))))))

(event `self.ClearBox.OnComponentBeginOverlap`
  (params (OverlappedComponent :type "PrimitiveComponent Object Reference") (OtherActor :type "Actor Object Reference") (OtherComp :type "PrimitiveComponent Object Reference") (OtherBodyIndex :type Integer) (bFromSweep :type Boolean) (SweepResult :type "HitResult Structure (by ref)"))
  ;[1 1 1] クリア判定
  (cast `/Game/BluePrints/Player/BP_FirstPersonCharacter` OtherActor)
  (bind _asbp_first_person_game_mode (cast `/Game/BluePrints/Framework/GameModes/BP_FirstPersonGameMode` (`GameplayStatics.GetGameMode`)))
  (`/Game/BluePrints/Framework/GameModes/BP_FirstPersonGameMode.GameClear_Event` _asbp_first_person_game_mode))

(fn `UserConstructionScript`
  (`parent.UserConstructionScript`))