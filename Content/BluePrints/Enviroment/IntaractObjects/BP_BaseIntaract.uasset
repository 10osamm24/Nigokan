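; BP_BaseIntaract is a base interactable object that shows an on-screen interact icon while the first-person character is within range.
; It creates a collapsed BPW_IntaractIcon widget on BeginPlay and toggles it through IntaractRounge overlap events.
; While the player is in range, Tick projects the range component's world location to screen space to position the icon.
; OnLooking_Event and UnLooking_Event are empty here.
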(event `self.ReceiveBeginPlay`
  ;[1 1 1] 初期化処理
  (bind _returnvalue (`|CreateWidget` "/Game/BluePrints/UI/InGame/BPW_IntaractIcon.BPW_IntaractIcon_C" (`HUD.GetOwningPlayerController` (`PlayerController.GetHUD` (`GameplayStatics.GetPlayerController` 0)))))
  (bind _output_get (set `self.intaractIcon` _returnvalue))
  (`UserWidget.AddToViewport` _output_get 0)
  (`Widget.SetVisibility` _output_get "Collapsed"))

(event `self.ReceiveTick`
  (params (DeltaSeconds :type "Float (single-precision)"))
  ;[1 1 1] 更新処理
  (`self.UpdateIntractIcon`))

(event `self.IntaractRounge.OnComponentBeginOverlap`
  (params (OverlappedComponent :type "PrimitiveComponent Object Reference") (OtherActor :type "Actor Object Reference") (OtherComp :type "PrimitiveComponent Object Reference") (OtherBodyIndex :type Integer) (bFromSweep :type Boolean) (SweepResult :type "HitResult Structure (by ref)"))
  ;[1 1 1] インタラクトアイコン表示
  (cast `/Game/BluePrints/Player/BP_FirstPersonCharacter` OtherActor)
  (set `self.isPlayerRounge` true)
  (`Widget.SetVisibility` (`self.intaractIcon`) "Visible"))

(event `self.IntaractRounge.OnComponentEndOverlap`
  (params (OverlappedComponent :type "PrimitiveComponent Object Reference") (OtherActor :type "Actor Object Reference") (OtherComp :type "PrimitiveComponent Object Reference") (OtherBodyIndex :type Integer))
  ;[1 1 1] インタラクトアイコン表示
  (cast `/Game/BluePrints/Player/BP_FirstPersonCharacter` OtherActor)
  (set `self.isPlayerRounge` false)
  (`Widget.SetVisibility` (`self.intaractIcon`) "Collapsed"))

(event `OnLooking_Event`)

(event `UnLooking_Event`)

(fn `UpdateIntractIcon`
  (bind _intaracticon (`self.intaractIcon`))
  (if (`self.isPlayerRounge`)
    (`Widget.SetVisibility` _intaracticon "Visible")
    (`UserWidget.SetPositionInViewport` _intaracticon (`PlayerController.ProjectWorldLocationToScreen` (`GameplayStatics.GetPlayerController` 0) (`SceneComponent.K2_GetComponentLocation` (`self.IntaractRounge`)) false) true)))

(fn `UserConstructionScript`)